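; BP_Trap is a trap actor made of three child-actor sniper rifles that spin in place and fire repeatedly.
; On BeginPlay it enables physics without gravity on each rifle's mesh, applies a different yaw angular impulse to each, and collects the rifles in an array.
; A looping one-second timer then calls FireShot on every rifle in that array.
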(event `self.ReceiveBeginPlay`
  (`|ExecutionSequence`
    (:`then_0`
      (bind _assniper_rifle (cast `SniperRifle` (`ChildActorComponent.ChildActor` (`self.FirstSniperRifle`))))
      (bind _staticmesh (`Item.StaticMesh` _assniper_rifle))
      (`PrimitiveComponent.SetSimulatePhysics` _staticmesh true)
      (`PrimitiveComponent.SetEnableGravity` _staticmesh false)
      (`PrimitiveComponent.AddAngularImpulseInRadians` _staticmesh (0.0 0.0 5.0) "None" true)
      (`KismetArrayLibrary.Array_AddUnique` (`self.SniperRifleArray`) _assniper_rifle))
    (:`then_1`
      (bind _assniper_rifle_2 (cast `SniperRifle` (`ChildActorComponent.ChildActor` (`self.SecondSniperRifle`))))
      (bind _staticmesh_2 (`Item.StaticMesh` _assniper_rifle_2))
      (`PrimitiveComponent.SetSimulatePhysics` _staticmesh_2 true)
      (`PrimitiveComponent.SetEnableGravity` _staticmesh_2 false)
      (`PrimitiveComponent.AddAngularImpulseInRadians` _staticmesh_2 (0.0 0.0 3.0) "None" true)
      (`KismetArrayLibrary.Array_AddUnique` (`self.SniperRifleArray`) _assniper_rifle_2))
    (:`then_2`
      (bind _assniper_rifle_3 (cast `SniperRifle` (`ChildActorComponent.ChildActor` (`self.ThirdSniperRifle`))))
      (bind _staticmesh_3 (`Item.StaticMesh` _assniper_rifle_3))
      (`PrimitiveComponent.SetSimulatePhysics` _staticmesh_3 true)
      (`PrimitiveComponent.SetEnableGravity` _staticmesh_3 false)
      (`PrimitiveComponent.AddAngularImpulseInRadians` _staticmesh_3 (0.0 0.0 -5.0) "None" true)
      (`KismetArrayLibrary.Array_AddUnique` (`self.SniperRifleArray`) _assniper_rifle_3))
    (:`then_3`
      (`KismetSystemLibrary.K2_SetTimerDelegate` (delegate `FireShotEvent`) 1.0 true))
    (:`then_4`
      (for _array_element (`self.SniperRifleArray`)
        (bind _staticmesh_4 (`Item.StaticMesh` _array_element))
        (`PrimitiveComponent.SetSimulatePhysics` _staticmesh_4 true)
        (`PrimitiveComponent.SetEnableGravity` _staticmesh_4 false)))))

(event `FireShotEvent`
  (for _array_element (`self.SniperRifleArray`)
    (`SniperRifle.FireShot` _array_element)))

(fn `UserConstructionScript`)